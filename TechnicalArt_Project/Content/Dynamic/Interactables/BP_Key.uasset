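; BP_Key is an interactable key pickup that advances the player's objective from finding the key to escaping.
; On BeginPlay it creates a WB_FindKey widget for player 0 and adds it to the viewport as the task display.
; Interacting calls PickUpKeyMessage on its referenced Door, destroys the key, and sets the widget's task text to "Escape".
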(event `/Game/Dynamic/Mechanics/BPI_Interact.Interact`
  (message `/Game/Dynamic/Mechanics/BPI_Door.Pick Up Key` (`self.Door`))
  (`self.K2_DestroyActor`)
  (`TextBlock.SetText` (`/Game/Dynamic/UI/WB_FindKey.Text_Task` (`self.WB_FindKey`)) "Escape"))

(event `self.ReceiveBeginPlay`
  (bind _returnvalue (`|CreateWidget` "/Game/Dynamic/UI/WB_FindKey.WB_FindKey_C" (`GameplayStatics.GetPlayerController` 0)))
  (bind _output_get (set `self.WB_FindKey` _returnvalue))
  (`UserWidget.AddToViewport` _output_get 0))

(fn `UserConstructionScript`)