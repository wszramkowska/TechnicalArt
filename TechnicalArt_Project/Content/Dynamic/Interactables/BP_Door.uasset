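; BP_Door is an interactable double door that opens and closes once its key has been picked up.
; PickUpKey sets HasKey, which Interact checks before a FlipFlop alternates between playing and reversing a timeline.
; The timeline swings DoorL and DoorR to mirrored 90-degree yaw rotations through a Lerp.
; A Box overlap shows and hides a Widget.
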(event `/Game/Dynamic/Mechanics/BPI_Interact.Interact`
  ;[1 1 1] Door opens if player has key
  (if (`self.Has Key?`)
    (`/Engine/EditorBlueprintResources/StandardMacros.FlipFlop`
      (:`A`
        (bind (_direction _door_track) (`Timeline|Door Timelinr` :!label _label)
          (:`Update`
            (bind _returnvalue (`KismetMathLibrary.Lerp` 0.0 90.0 _door_track))
            (`SceneComponent.K2_SetRelativeRotation` (`self.DoorL`) (`KismetMathLibrary.MakeRotator` 0.0 0.0 _returnvalue) false false)
            (`SceneComponent.K2_SetRelativeRotation` (`self.DoorR`) (`KismetMathLibrary.MakeRotator` 0.0 0.0 (* _returnvalue -1.0)) false false))))
      (:`B`
        (goto _label :!via `Reverse`)))))

(event `/Game/Dynamic/Mechanics/BPI_Door.Pick Up Key`
  ;[1 1 1] Door opens if player has key
  (set `self.Has Key?` true))

(event `self.Box.OnComponentBeginOverlap`
  (params (OverlappedComponent :type "PrimitiveComponent Object Reference") (OtherActor :type "Actor Object Reference") (OtherComp :type "PrimitiveComponent Object Reference") (OtherBodyIndex :type Integer) (bFromSweep :type Boolean) (SweepResult :type "HitResult Structure (by ref)"))
  (`SceneComponent.SetVisibility` (`self.Widget`) true false))

(event `self.Box.OnComponentEndOverlap`
  (params (OverlappedComponent :type "PrimitiveComponent Object Reference") (OtherActor :type "Actor Object Reference") (OtherComp :type "PrimitiveComponent Object Reference") (OtherBodyIndex :type Integer))
  (`SceneComponent.SetVisibility` (`self.Widget`) false false))

(fn `UserConstructionScript`)