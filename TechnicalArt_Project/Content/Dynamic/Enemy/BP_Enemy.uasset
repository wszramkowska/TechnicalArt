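; Zombie-style enemy that wanders randomly, chases and melee-attacks pawns it sees, driven by PawnSensing and AIMoveTo without a behavior tree.
; Sighting triggers a sprint and chase, while a retriggerable delay drops it back to walking patrol once sightings stop.
; Reaching the target plays a random, DoOnce-gated attack montage with a scream.
; The montage notify applies damage to pawns in a sphere overlap, with a debug sphere drawn.
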(event `self.ReceiveBeginPlay`
  (`self.MoveToRandomLocation`))

(event `MoveToRandomLocation`
  ;[1 1 1] Patrol
  (bind _randomlocation (`NavigationSystemV1.K2_GetRandomLocationInNavigableRadius` (`self.K2_GetActorLocation`) 1000.0 null null))
  (`|AIMoveTo` self _randomlocation null
    (:`OnSuccess`
      (`self.MoveToRandomLocation`))))

(event `CanSprintAgain`
  ;[1 1 1] Chase
  (goto _label :!via `Reset`))

(event `self.PawnSensing.OnSeePawn`
  (params (Pawn :type "Pawn Object Reference"))
  ;[1 1 1] Chase
  (`|ExecutionSequence`
    (:`then_0`
      (`/Engine/EditorBlueprintResources/StandardMacros.DoOnce` false :!label _label
        (:`Completed`
          (set `CharacterMovementComponent.MaxWalkSpeed` 500.0 (`self.CharacterMovement`)))))
    (:`then_1`
      (`|AIMoveTo` self (0.0 0.0 0.0) Pawn
        (:`then`
          (`KismetSystemLibrary.RetriggerableDelay` 2.0)
          (set `CharacterMovementComponent.MaxWalkSpeed` 130.0 (`self.CharacterMovement`))
          (`self.CanSprintAgain`)
          (`self.MoveToRandomLocation`))
        (:`OnSuccess`
          (`self.Attack`))))))

(event `Attack`
  (bind _attackanims (`self.AttackAnims`))
  ;[1 1 1] Attack Anim
  (`/Engine/EditorBlueprintResources/StandardMacros.DoOnce` false :!label _label_2
    (:`Completed`
      (`|PlayMontage` (`self.Mesh`) (`|GetArrayItem` _attackanims (`KismetMathLibrary.RandomInteger` (`KismetArrayLibrary.Array_Length` _attackanims)))
        (:`then`
          (`GameplayStatics.PlaySound2D` "/Game/Static/Audio/Zombie-scream.Zombie-scream" 20.0 1.0 0.0 null null))
        (:`OnCompleted`
          (`CharacterMovementComponent.SetMovementMode` (`self.CharacterMovement`) "MOVE_Walking" 0 :!label _label_3)
          (goto _label_2 :!via `Reset`))
        (:`OnInterrupted`
          (`KismetSystemLibrary.Delay` 1.0)
          (goto _label_3))
        (:`OnNotifyBegin`
          (`self.DealDamage`))))))

(event `DealDamage`
  (bind _returnvalue (`SceneComponent.K2_GetComponentLocation` (`self.AttackRadius`)))
  ;[1 1 1] Deal Damage
  (bind _outactors (`KismetSystemLibrary.SphereOverlapActors` _returnvalue (`self.AttackRange`) (`|MakeArray` "ObjectTypeQuery3" :!type "EObjectTypeQuery Enum") "/Script/Engine.Actor" (`|MakeArray` self :!type "Actor Object Reference")))
  (`KismetSystemLibrary.DrawDebugSphere` _returnvalue (`self.AttackRange`) 12 (struct :`R` 0.384487 :`B` 0.546875 :`A` 1.0) 2.0)
  (for _array_element _outactors
    (`GameplayStatics.ApplyDamage` _array_element (`self.Base Damage`) (`self.GetController`) self "/Script/Engine.DamageType")))

(fn `UserConstructionScript`)