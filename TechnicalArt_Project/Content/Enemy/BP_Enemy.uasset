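; Zombie enemy Blueprint that wanders, chases the player on sight and plays a melee attack montage.
; An EnemyState value drives per-Tick AI moves across Patroling, Chasing and Attacking, alongside a self-repeating random-point patrol.
; Pawn sensing starts the chase, with a DoOnce for sprint speed and a retriggerable delay that restores walk speed and wandering.
; The Attack event runs a socket sphere trace to apply damage; AttackPlayer is an empty stub.
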(event `self.ReceiveBeginPlay`
  (`self.MoveToRandomLocation`))

(event `MoveToRandomLocation`
  ;[1 1 1] Patrol
  (set `self.EnemyState` "NewEnumerator1")
  (`|AIMoveTo` self (`NavigationSystemV1.K2_GetRandomReachablePointInRadius` (`self.K2_GetActorLocation`) 1000.0 null null) null
    (:`OnSuccess`
      (`self.MoveToRandomLocation`))))

(event `CanSprintAgain`
  ;[1 1 1] Chase
  (goto _label :!via `Reset`))

(event `self.PawnSensing.OnSeePawn`
  (params (Pawn :type "Pawn Object Reference"))
  (if (== Pawn (`GameplayStatics.GetPlayerPawn` 0))
    (set `self.EnemyState` "NewEnumerator0")
    ;[1 1 1] Chase
    (`|ExecutionSequence`
      (:`then_0`
        (`/Engine/EditorBlueprintResources/StandardMacros.DoOnce` false :!label _label
          (:`Completed`
            (set `CharacterMovementComponent.MaxWalkSpeed` 450.0 (`self.CharacterMovement`)))))
      (:`then_1`
        (`|AIMoveTo` self (0.0 0.0 0.0) null 150.0
          (:`then`
            (`KismetSystemLibrary.RetriggerableDelay` 2.0)
            (set `CharacterMovementComponent.MaxWalkSpeed` 130.0 (`self.CharacterMovement`))
            (`self.CanSprintAgain`)
            (`self.MoveToRandomLocation`))
          (:`OnSuccess`
            (`self.AttackPlayer`)))))))

(event `/Game/Interfaces/I_Attack.Attack`
  (`self.AttackTrace`))

(event `AttackPlayer`)

(event `self.ReceiveTick`
  (params (DeltaSeconds :type "Float (single-precision)"))
  (`self.Handle Behaviours`))

(event `Handle Behaviours`
  (switch `/Game/Enemy/EnemyStates/E_EnemyStates` (`self.EnemyState`)
    (:`NewEnumerator0`
      (`|AIMoveTo` self (0.0 0.0 0.0) (`self.Target`) 250.0
        (:`OnSuccess`
          (bind _returnvalue (`self.PlayAnimMontage` "/Game/Enemy/AnimationMontages/Zombie_Attack1_Montage.Zombie_Attack1_Montage"))
          (set `self.EnemyState` "NewEnumerator3"))))
    (:`NewEnumerator1`
      (bind _patrollocation (`self.Patrol`))
      (`|AIMoveTo` self _patrollocation null 150.0))
    (:`NewEnumerator3`
      (if (> _returnvalue 3.83)
        (set `self.EnemyState` "NewEnumerator0")))))

(fn `AttackTrace`
  (bind _returnvalue (`SceneComponent.GetSocketLocation` (`self.Mesh`) "AttackSocket"))
  (`KismetSystemLibrary.SphereTraceMultiForObjects` :`Start` _returnvalue :`End` _returnvalue :`Radius` 40.0 :`ObjectTypes` (`|MakeArray` "ObjectTypeQuery3" :!type "EObjectTypeQuery Enum") :`DrawDebugType` "ForOneFrame")
  (`GameplayStatics.ApplyDamage` null 10.0))

(fn `Chase`
  (returns (IsNearPlayer :type Boolean) (PawnLocation :type "Vector Structure"))
  (bind _returnvalue (`self.K2_GetActorLocation`))
  (bind _outhit (`KismetSystemLibrary.LineTraceSingle` :`Start` (`self.K2_GetActorLocation` self) :`End` _returnvalue :`TraceChannel` "TraceTypeQuery1" :`DrawDebugType` "ForDuration"))
  (if (== (`self.Target`) (`.HitActor` (`GameplayStatics.BreakHitResult` _outhit)))
    (return (<= (`.Distance` (`GameplayStatics.BreakHitResult` _outhit)) 50.0) _returnvalue)))

(fn `Patrol`
  (returns (PatrolLocation :type "Vector Structure"))
  (return (`NavigationSystemV1.K2_GetRandomReachablePointInRadius` (`self.K2_GetActorLocation`) 1000.0 null null)))

(fn `UserConstructionScript`)